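; Player controller that routes directional input for two local players to the game manager.
; On BeginPlay it adds the Enhanced Input mapping context and caches the first BP_GameManager found in the level.
; Each player's up, down, left and right actions call the manager's PressCheck with a WASD key letter and player number, so one controller serves both players.
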(event `self.ReceiveBeginPlay`
  (`EnhancedInputSubsystemInterface.AddMappingContext` (pcsubsystem `EnhancedInputLocalPlayerSubsystem` self) "/Game/MarcContents/Input/IA_Mapping.IA_Mapping" 0 (struct))
  (bind _outactors (`GameplayStatics.GetAllActorsOfClass` "/Game/MarcContents/Blueprints/BP_GameManager.BP_GameManager_C"))
  (set `self.GameManager` (`|GetArrayItem` _outactors)))

(event `EnhancedInput|/Game/MarcContents/Input/IA_Up1`
  (params (ActionValue :type Boolean) (ElapsedSeconds :type "Float (double-precision)") (TriggeredSeconds :type "Float (double-precision)") (InputAction :type "InputAction Object Reference" :default "/Game/MarcContents/Input/IA_Up1.IA_Up1"))
  (:`Triggered`
    (`/Game/MarcContents/Blueprints/BP_GameManager.PressCheck` (`self.GameManager`) "W" 1)))

(event `EnhancedInput|/Game/MarcContents/Input/IA_Up2`
  (params (ActionValue :type Boolean) (ElapsedSeconds :type "Float (double-precision)") (TriggeredSeconds :type "Float (double-precision)") (InputAction :type "InputAction Object Reference" :default "/Game/MarcContents/Input/IA_Up2.IA_Up2"))
  (:`Triggered`
    (`/Game/MarcContents/Blueprints/BP_GameManager.PressCheck` (`self.GameManager`) "W" 2)))

(event `EnhancedInput|/Game/MarcContents/Input/IA_Left1`
  (params (ActionValue :type Boolean) (ElapsedSeconds :type "Float (double-precision)") (TriggeredSeconds :type "Float (double-precision)") (InputAction :type "InputAction Object Reference" :default "/Game/MarcContents/Input/IA_Left1.IA_Left1"))
  (:`Triggered`
    (`/Game/MarcContents/Blueprints/BP_GameManager.PressCheck` (`self.GameManager`) "A" 1)))

(event `EnhancedInput|/Game/MarcContents/Input/IA_Left2`
  (params (ActionValue :type Boolean) (ElapsedSeconds :type "Float (double-precision)") (TriggeredSeconds :type "Float (double-precision)") (InputAction :type "InputAction Object Reference" :default "/Game/MarcContents/Input/IA_Left2.IA_Left2"))
  (:`Triggered`
    (`/Game/MarcContents/Blueprints/BP_GameManager.PressCheck` (`self.GameManager`) "A" 2)))

(event `EnhancedInput|/Game/MarcContents/Input/IA_Down1`
  (params (ActionValue :type Boolean) (ElapsedSeconds :type "Float (double-precision)") (TriggeredSeconds :type "Float (double-precision)") (InputAction :type "InputAction Object Reference" :default "/Game/MarcContents/Input/IA_Down1.IA_Down1"))
  (:`Triggered`
    (`/Game/MarcContents/Blueprints/BP_GameManager.PressCheck` (`self.GameManager`) "S" 1)))

(event `EnhancedInput|/Game/MarcContents/Input/IA_Down2`
  (params (ActionValue :type Boolean) (ElapsedSeconds :type "Float (double-precision)") (TriggeredSeconds :type "Float (double-precision)") (InputAction :type "InputAction Object Reference" :default "/Game/MarcContents/Input/IA_Down2.IA_Down2"))
  (:`Triggered`
    (`/Game/MarcContents/Blueprints/BP_GameManager.PressCheck` (`self.GameManager`) "S" 2)))

(event `EnhancedInput|/Game/MarcContents/Input/IA_Right1`
  (params (ActionValue :type Boolean) (ElapsedSeconds :type "Float (double-precision)") (TriggeredSeconds :type "Float (double-precision)") (InputAction :type "InputAction Object Reference" :default "/Game/MarcContents/Input/IA_Right1.IA_Right1"))
  (:`Triggered`
    (`/Game/MarcContents/Blueprints/BP_GameManager.PressCheck` (`self.GameManager`) "D" 1)))

(event `EnhancedInput|/Game/MarcContents/Input/IA_Right2`
  (params (ActionValue :type Boolean) (ElapsedSeconds :type "Float (double-precision)") (TriggeredSeconds :type "Float (double-precision)") (InputAction :type "InputAction Object Reference" :default "/Game/MarcContents/Input/IA_Right2.IA_Right2"))
  (:`Triggered`
    (`/Game/MarcContents/Blueprints/BP_GameManager.PressCheck` (`self.GameManager`) "D" 2)))

(fn `UserConstructionScript`)
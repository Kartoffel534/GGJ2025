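; BP_GameManager runs a two-player potion game where players race to type randomized three-key codes.
; ResetPotion rolls a unique code and two random stat values for each of three potions, refreshed every five seconds or on claim, and notifies BP_UI.
; PressCheck matches each player's last three keys, applying potion values and counting claims.
; Reaching WinCondition wins, a stat hitting ±LoseCondition loses, and GameWin locks input and shows the winner.
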(event `self.ReceiveBeginPlay`
  (`self.ResetPotion` 1)
  (`self.ResetPotion` 2)
  (`self.ResetPotion` 3)
  (set `self.InputAllowed` true))

(event `self.ReceiveTick`
  (params (DeltaSeconds :type "Float (single-precision)"))
  (bind _output_get (set `self.ResetTimer` (+ DeltaSeconds (`self.ResetTimer`))))
  (if (>= _output_get 5.0)
    (set `self.ResetTimer` (- (`self.ResetTimer`) 5.0))
    (`self.ResetPotion` 1)
    (`self.ResetPotion` 2)
    (`self.ResetPotion` 3)))

(fn `GameWin`
  (params (Winner :type Integer))
  (`GameplayStatics.PlaySound2D` "/Game/Sound/Postive_Bubble_Jingle_01_2.Postive_Bubble_Jingle_01_2" 1.0 1.0 0.0 null null)
  (bind _foundwidgets (`WidgetBlueprintLibrary.GetAllWidgetsOfClass` "/Game/MarcContents/UI/BP_UI.BP_UI_C" false))
  (bind _output_get (set `self.UI_Ref` (`|GetArrayItem` _foundwidgets)))
  (set `self.InputAllowed` false)
  (`/Game/MarcContents/UI/BP_UI.WinnerTextAppear` _output_get Winner))

(fn `PressCheck`
  (params (Key :type String) (Player :type Integer))
  (bind _losecondition (`self.LoseCondition`))
  (bind _losecondition_2 (`self.LoseCondition`))
  (bind _losecondition_3 (`self.LoseCondition`))
  (bind _losecondition_4 (`self.LoseCondition`))
  (if (`self.InputAllowed`)
    (if (== 1 Player)
      (if (< (`KismetStringLibrary.Len` (`self.CheckStringP1`)) 3)
        (set `self.CheckStringP1` (`KismetStringLibrary.Concat_StrStr` (`self.CheckStringP1`) Key))
        (if (== (`KismetStringLibrary.Len` (`self.CheckStringP1`)) 3)
          (if (`KismetStringLibrary.EqualEqual_StrStr` (`self.InputValue1`) (`self.CheckStringP1`)) :!label _label
            (set `self.CheckStringP1` "")
            (set `self.Player1A` (+ (`self.Player1A`) (`self.PotionValue1A`)))
            (set `self.Player1B` (+ (`self.Player1B`) (`self.PotionValue1B`)))
            (`self.ResetPotion` 1)
            (`GameplayStatics.PlaySound2D` "/Game/Sound/8bit_Bubble_magic_shoot_01_1.8bit_Bubble_magic_shoot_01_1" 1.0 1.0 0.0 null null :!label _label_2)
            (set `self.Player1Potions` (+ (`self.Player1Potions`) 1))
            (if (== (`self.WinCondition`) (`self.Player1Potions`))
              (`self.GameWin` 1 :!label _label_3)
              (elif (not (and (`KismetMathLibrary.InRange_IntInt` (`self.Player1B`) (- 0 _losecondition) _losecondition false false) (`KismetMathLibrary.InRange_IntInt` (`self.Player1A`) (- 0 _losecondition_2) _losecondition_2 false false)))
                (`self.GameWin` 2 :!label _label_4)))
            (elif (`KismetStringLibrary.EqualEqual_StrStr` (`self.InputValue2`) (`self.CheckStringP1`))
              (set `self.CheckStringP1` "")
              (set `self.Player1A` (+ (`self.Player1A`) (`self.PotionValue2A`)))
              (set `self.Player1B` (+ (`self.Player1B`) (`self.PotionValue2B`)))
              (`self.ResetPotion` 2)
              (goto _label_2)
              (elif (`KismetStringLibrary.EqualEqual_StrStr` (`self.InputValue3`) (`self.CheckStringP1`))
                (set `self.CheckStringP1` "")
                (set `self.Player1A` (+ (`self.Player1A`) (`self.PotionValue3A`)))
                (set `self.Player1B` (+ (`self.Player1B`) (`self.PotionValue3B`)))
                (`self.ResetPotion` 3)
                (goto _label_2)))))
        (else
          (set `self.CheckStringP1` (`KismetStringLibrary.Concat_StrStr` (`KismetStringLibrary.Right` (`self.CheckStringP1`) 2) Key))
          (goto _label)))
      (elif (< (`KismetStringLibrary.Len` (`self.CheckStringP2`)) 3)
        (set `self.CheckStringP2` (`KismetStringLibrary.Concat_StrStr` (`self.CheckStringP2`) Key))
        (if (== (`KismetStringLibrary.Len` (`self.CheckStringP2`)) 3)
          (if (`KismetStringLibrary.EqualEqual_StrStr` (`self.InputValue1`) (`self.CheckStringP2`)) :!label _label_5
            (set `self.CheckStringP2` "")
            (set `self.Player2A` (+ (`self.Player2A`) (`self.PotionValue1A`)))
            (set `self.Player2B` (+ (`self.Player2B`) (`self.PotionValue1B`)))
            (`self.ResetPotion` 1)
            (`GameplayStatics.PlaySound2D` "/Game/Sound/8bit_Bubble_magic_shoot_01_1.8bit_Bubble_magic_shoot_01_1" 1.0 1.0 0.0 null null :!label _label_6)
            (set `self.Player2Potions` (+ (`self.Player2Potions`) 1))
            (if (== (`self.WinCondition`) (`self.Player2Potions`))
              (goto _label_4)
              (elif (not (and (`KismetMathLibrary.InRange_IntInt` (`self.Player2A`) (- 0 _losecondition_3) _losecondition_3 false false) (`KismetMathLibrary.InRange_IntInt` (`self.Player2B`) (- 0 _losecondition_4) _losecondition_4 false false)))
                (goto _label_3)))
            (elif (`KismetStringLibrary.EqualEqual_StrStr` (`self.InputValue2`) (`self.CheckStringP2`))
              (set `self.CheckStringP2` "")
              (set `self.Player2A` (+ (`self.Player2A`) (`self.PotionValue2A`)))
              (set `self.Player2B` (+ (`self.Player2B`) (`self.PotionValue2B`)))
              (`self.ResetPotion` 2)
              (goto _label_6)
              (elif (`KismetStringLibrary.EqualEqual_StrStr` (`self.InputValue3`) (`self.CheckStringP2`))
                (set `self.CheckStringP2` "")
                (set `self.Player2A` (+ (`self.Player2A`) (`self.PotionValue3A`)))
                (set `self.Player2B` (+ (`self.Player2B`) (`self.PotionValue3B`)))
                (`self.ResetPotion` 3)
                (goto _label_6)))))
        (else
          (set `self.CheckStringP2` (`KismetStringLibrary.Concat_StrStr` (`KismetStringLibrary.Right` (`self.CheckStringP2`) 2) Key))
          (goto _label_5))))))

(fn `ResetPotion`
  (params (Number :type Integer))
  (bind _returnvalue (`KismetMathLibrary.RandomIntegerInRange` 1 2))
  (bind _returnvalue_2 (`KismetMathLibrary.RandomIntegerInRange` 1 2))
  (bind _returnvalue_3 (`KismetMathLibrary.RandomIntegerInRange` 1 2))
  (bind _returnvalue_4 (`KismetMathLibrary.RandomIntegerInRange` 1 2))
  (bind _returnvalue_5 (`KismetMathLibrary.RandomIntegerInRange` 1 2))
  (bind _returnvalue_6 (`KismetMathLibrary.RandomIntegerInRange` 1 2))
  (if (== Number 1)
    (set `self.InputValue1` "")
    (for _ (range 3)
      (set `self.InputValue1` (`KismetStringLibrary.Concat_StrStr` (`|GetArrayItem` (`self.InputOptions`) (`KismetMathLibrary.RandomIntegerInRange` 0 3)) (`self.InputValue1`))))
    (bind _foundwidgets (`WidgetBlueprintLibrary.GetAllWidgetsOfClass` "/Game/MarcContents/UI/BP_UI.BP_UI_C" false))
    (message `/Game/Blueprints/TestInterface.UI_Magic` _foundwidgets)
    (if (or (`KismetStringLibrary.EqualEqual_StrStr` (`self.InputValue1`) (`self.InputValue2`)) (`KismetStringLibrary.EqualEqual_StrStr` (`self.InputValue1`) (`self.InputValue3`)))
      (`self.ResetPotion` 1)
      (else
        (if (== (`KismetMathLibrary.RandomIntegerInRange` 0 1) 0)
          (set `self.PotionValue1A` _returnvalue_3)
          (else
            (bind _result (`/Engine/EditorBlueprintResources/StandardMacros.NegateInt` _returnvalue_3)
              (:`  `
                (set `self.PotionValue1A` _result)))))
        (if (== (`KismetMathLibrary.RandomIntegerInRange` 0 1) 0)
          (set `self.PotionValue1B` _returnvalue_4)
          (else
            (bind _result_2 (`/Engine/EditorBlueprintResources/StandardMacros.NegateInt` _returnvalue_4)
              (:`  `
                (set `self.PotionValue1B` _result_2)))))))
    (elif (== Number 2)
      (set `self.InputValue2` "")
      (for _ (range 3)
        (set `self.InputValue2` (`KismetStringLibrary.Concat_StrStr` (`|GetArrayItem` (`self.InputOptions`) (`KismetMathLibrary.RandomIntegerInRange` 0 3)) (`self.InputValue2`))))
      (bind _foundwidgets_2 (`WidgetBlueprintLibrary.GetAllWidgetsOfClass` "/Game/MarcContents/UI/BP_UI.BP_UI_C" false))
      (message `/Game/Blueprints/TestInterface.UI_Magic1` _foundwidgets_2)
      (if (or (`KismetStringLibrary.EqualEqual_StrStr` (`self.InputValue1`) (`self.InputValue2`)) (`KismetStringLibrary.EqualEqual_StrStr` (`self.InputValue2`) (`self.InputValue3`)))
        (`self.ResetPotion` 2)
        (else
          (if (== (`KismetMathLibrary.RandomIntegerInRange` 0 1) 0)
            (set `self.PotionValue2A` _returnvalue_5)
            (else
              (bind _result_3 (`/Engine/EditorBlueprintResources/StandardMacros.NegateInt` _returnvalue_5)
                (:`  `
                  (set `self.PotionValue2A` _result_3)))))
          (if (== (`KismetMathLibrary.RandomIntegerInRange` 0 1) 0)
            (set `self.PotionValue2B` _returnvalue_6)
            (else
              (bind _result_4 (`/Engine/EditorBlueprintResources/StandardMacros.NegateInt` _returnvalue_6)
                (:`  `
                  (set `self.PotionValue2B` _result_4)))))))
      (elif (== Number 3)
        (set `self.InputValue3` "")
        (for _ (range 3)
          (set `self.InputValue3` (`KismetStringLibrary.Concat_StrStr` (`|GetArrayItem` (`self.InputOptions`) (`KismetMathLibrary.RandomIntegerInRange` 0 3)) (`self.InputValue3`))))
        (bind _foundwidgets_3 (`WidgetBlueprintLibrary.GetAllWidgetsOfClass` "/Game/MarcContents/UI/BP_UI.BP_UI_C" false))
        (message `/Game/Blueprints/TestInterface.UI_Magic2` _foundwidgets_3)
        (if (or (`KismetStringLibrary.EqualEqual_StrStr` (`self.InputValue3`) (`self.InputValue2`)) (`KismetStringLibrary.EqualEqual_StrStr` (`self.InputValue1`) (`self.InputValue3`)))
          (`self.ResetPotion` 3)
          (else
            (if (== (`KismetMathLibrary.RandomIntegerInRange` 0 1) 0)
              (set `self.PotionValue3A` _returnvalue_2)
              (else
                (bind _result_5 (`/Engine/EditorBlueprintResources/StandardMacros.NegateInt` _returnvalue_2)
                  (:`  `
                    (set `self.PotionValue3A` _result_5)))))
            (if (== (`KismetMathLibrary.RandomIntegerInRange` 0 1) 0)
              (set `self.PotionValue3B` _returnvalue)
              (else
                (bind _result_6 (`/Engine/EditorBlueprintResources/StandardMacros.NegateInt` _returnvalue)
                  (:`  `
                    (set `self.PotionValue3B` _result_6)))))))))))

(fn `UserConstructionScript`)